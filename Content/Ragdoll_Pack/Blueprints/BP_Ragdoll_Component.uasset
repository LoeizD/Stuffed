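; BP_Ragdoll_Component is a component meant to boot a ragdoll actor for the pawn that owns it.
; Its disconnected logic spawns a BP_Ragdoll_Actor, passes it the component's strength, force and profile settings through BootValues, then calls BootEvents with the owning Pawn.
; BeginPlay has nothing wired to it, so none of this setup runs as the graph stands.
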(event `self.ReceiveBeginPlay`
  ;[1 1 1] boot ragdoll actor
)