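; Sound actor for TheMule that plays a short "Fourrage" sound effect and toggles an alarm siren, both as 2D audio.
; PlaySOund starts the loopable clip at a random offset for variation, replaces any previous instance, then stops it after a brief delay.
; Alarm spawns the siren when switched on, keeping its audio component so it can be stopped when switched off.
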(event `PlaySOund`
  (bind _returnvalue (`GameplayStatics.SpawnSound2D` "/Game/TheMule/Sound/fourrage_loopable16.fourrage_loopable16" 13.0 1.0 (`KismetMathLibrary.RandomFloatInRange` 0.0 6.0)))
  (`AudioComponent.Stop` (`self.Fourga`))
  (bind _output_get (set `self.Fourga` _returnvalue))
  (`KismetSystemLibrary.Delay` 0.5)
  (`AudioComponent.Stop` _output_get))

(event `Alarm`
  (params (On :type Boolean))
  (bind _newvar_0 (`self.NewVar_0`))
  (if On
    (bind _returnvalue (`GameplayStatics.SpawnSound2D` "/Game/TheMule/Sound/371179__samsterbirdies__siren16.371179__samsterbirdies__siren16"))
    (set `self.NewVar_0` _returnvalue)
    (else
      (`/Engine/EditorBlueprintResources/StandardMacros.IsValid` _newvar_0
        (:`Is Valid`
          (`AudioComponent.Stop` _newvar_0))))))

(fn `UserConstructionScript`)